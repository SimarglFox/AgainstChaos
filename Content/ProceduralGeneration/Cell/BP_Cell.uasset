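; BP_Cell is a procedural-generation map cell that moves between infected, fighting, temporarily open and purified states.
; Player overlap with an infected cell scales SpawnerComponent enemy counts by cleared cells, raises blocking walls and signals SoundController.
; When the spawner clears, walls drop, then the cell reinfects after a delay unless purified.
; Building enough torches purifies it, swapping grass materials, disabling post-process and crediting the player.
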(event Clear(SpawnerComponent)
  (CallFunction|SetWallVisibility false "ECR_Ignore")
  (Variables|Default|SetCellState "NewEnumerator3")
  (Utilities|FlowControl|Delay 15.0)
  (if (Utilities|Enum|NotEqual(Enum) (Variables|Default|GetCellState) "NewEnumerator2")
    (CallFunction|Infect)))

(event OnComponentBeginOverlap(ZoneTrigger)
  (params (OverlappedComponent :type Primitive%20Component%20Object%20Reference) (OtherActor :type Actor%20Object%20Reference) (OtherComp :type Primitive%20Component%20Object%20Reference) (OtherBodyIndex :type Integer) (bFromSweep :type Boolean) (SweepResult :type Hit%20Result%20Structure%20%28by%20ref%29))
  (bind _spawnercomponent (Variables|Default|GetSpawnerComponent))
  (if (Utilities|Enum|Equal(Enum) (Variables|Default|GetCellState) "NewEnumerator0")
    (bind _asfirst_person_character (Utilities|Casting|CastToFirstPersonCharacter OtherActor))
    (Utilities|FlowControl|Sequence
      (:then_0
        (Variables|/Game/EnemyBase/SpawnerComponent.SpawnerComponent_C|SetEnemyCount _spawnercomponent (* (Variables|/Game/FirstPersonBP/Blueprints/FirstPersonCharacter.FirstPersonCharacter_C|GetCellCleared _asfirst_person_character) 10))
        (Variables|/Game/EnemyBase/SpawnerComponent.SpawnerComponent_C|SetMaxSpawned _spawnercomponent (* (Variables|/Game/FirstPersonBP/Blueprints/FirstPersonCharacter.FirstPersonCharacter_C|GetCellCleared _asfirst_person_character) 5)))
      (:then_1
        (CallFunction|ActivateRoom)
        (bind _returnvalue (Actor|GetActorOfClass "/Game/Audio/SoundController.SoundController_C"))
        (Default|FightBegin _returnvalue)))))

(event Custom|BuildTorch
  (bind _result (Math|Integer|IncrementInt (Variables|Default|GetCurrentTorchCount))
    (:%20%20
      (if (== _result (Variables|Default|GetHeededTorches))
        (CallFunction|Clear)
        (bind _returnvalue (Actor|GetActorOfClass "/Game/FirstPersonBP/Blueprints/FirstPersonCharacter.FirstPersonCharacter_C"))
        (Default|CellCleared _returnvalue)))))

(fn ConstructionScript)

(fn Clear
  (CallFunction|SetWallVisibility false "ECR_Ignore")
  (CallFunction|SetMaterials (Variables|Default|GetPureGrass) (Variables|Default|GetPureFoliageGrassMat))
  (Variables|/Script/Engine.PostProcessComponent|SetbEnabled (Variables|Default|GetPostProcess) false)
  (Variables|Default|SetCellState "NewEnumerator2"))

(fn SetWallVisibility
  (params (NewVisibility :type Boolean) (CollisionResponce :type ECollisionResponse%20Enum :default "ECR_Ignore"))
  (for _array_element (Components|GetChildrenComponents (Variables|Default|GetWall) false)
    (bind _asstatic_mesh_component (Utilities|Casting|CastToStaticMeshComponent _array_element))
    (Rendering|SetVisibility _asstatic_mesh_component NewVisibility false)
    (Collision|SetCollisionResponsetoAllChannels _asstatic_mesh_component CollisionResponce)))

(fn ActivateRoom
  (CallFunction|SetMaterials (Variables|Default|GetInfectedGrass) (Variables|Default|GetInfectedFoliageGrassMat))
  (CallFunction|SetWallVisibility true "ECR_Block")
  (Default|BeginFight (Variables|Default|GetSpawnerComponent))
  (Variables|Default|SetCellState "NewEnumerator1"))

(fn CanBuild
  (return (< (Variables|Default|GetCurrentBuildCount) (Variables|Default|GetMaxBuildCount))))

(fn SetMaterials
  (params (PlathormGrassMat :type Material%20Interface%20Object%20Reference) (FoliageGrassMat :type Material%20Interface%20Object%20Reference))
  (Rendering|Material|SetMaterial (Variables|Default|GetPlatform) 0 PlathormGrassMat)
  (Rendering|Material|SetMaterial (Variables|Default|GetGrass) 0 FoliageGrassMat))

(fn Infect
  (CallFunction|SetMaterials (Variables|Default|GetInfectedGrass) (Variables|Default|GetInfectedFoliageGrassMat))
  (CallFunction|SetWallVisibility true "ECR_Ignore")
  (Variables|Default|SetCellState "NewEnumerator0"))