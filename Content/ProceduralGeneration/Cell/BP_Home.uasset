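; BP_Home is a procedural generation cell that serves as the player's starting spot.
; On BeginPlay it runs the parent logic, then teleports player character 0 to the X and Y of its Platform component at a fixed height.
; The construction script only calls the parent, and the overlap and tick events are disabled stubs.
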(event EventBeginPlay
  (bind _platform (Variables|Default|GetPlatform))
  (bind _returnvalue (Transformation|GetWorldLocation _platform))
  (|CallParentFunction)
  (Transformation|SetActorLocation (Game|GetPlayerCharacter 0) (Math|Vector|MakeVector (.x _returnvalue) (.y _returnvalue) 1e+02) false true))

(event Collision|EventActorBeginOverlap
  (params (OtherActor :type Actor%20Object%20Reference))
  (|CallParentFunction OtherActor) ; This node is disabled and will not be called.\nDrag off pins to build functionality.
)

(event EventTick
  (params (DeltaSeconds :type Float%20%28single-precision%29))
  (|CallParentFunction DeltaSeconds) ; This node is disabled and will not be called.\nDrag off pins to build functionality.
)

(fn ConstructionScript
  (|CallParentFunction))