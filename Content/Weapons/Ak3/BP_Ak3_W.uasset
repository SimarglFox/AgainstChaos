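; AK3 weapon Blueprint, built on a parent class, that handles firing and reloading.
; Shot, blocked during reloads, chains montages on the player's hands and weapon mesh, then spawns a bullet and shell casing and decrements ammo.
; Reload plays paired montages, holding a Reloading flag until the weapon montage blends out and ammo refills; without a valid player, it refills immediately.
; Hit damage is deferred to the parent.
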(event Custom|SpawnBulletCase
  (Game|SpawnActorfromClass "/Game/Weapons/Ak3/BP_BulletCase.BP_BulletCase_C" (Transformation|GetWorldTransform (Variables|Default|GetBulletCase)) "Undefined" 0 0))

(event EventHitDamageEvent
  (|CallParentFunction))

(event EventShot
  (if (not (Variables|Default|GetReloading))
    (Animation|Montage|PlayMontage (Variables|/Game/FirstPersonBP/Blueprints/FirstPersonCharacter.FirstPersonCharacter_C|GetHands (Variables|Default|GetPlayer)) "/Game/Animations/Ak3/Ak3_Shot_Montage.Ak3_Shot_Montage"
      (:then
        (Animation|Montage|PlayMontage (Variables|Default|GetWeapon) "/Game/Animations/WeaponAnimations/Ak3/Ak3_Weapon_Shot_Montage.Ak3_Weapon_Shot_Montage"
          (:then
            (CallFunction|SpawnBullet "/Game/Weapons/Revolver/BP_Bullet.BP_Bullet_C")
            (CallFunction|SpawnBulletCase)
            (Math|Integer|DecrementInt (Variables|Default|GetAmmo))))))))

(event EventReload
  (bind _player (Variables|Default|GetPlayer))
  (if (not (Variables|Default|GetReloading))
    (Utilities|IsValid _player
      (:Is%20Valid
        (Animation|Montage|PlayMontage (Variables|/Game/FirstPersonBP/Blueprints/FirstPersonCharacter.FirstPersonCharacter_C|GetHands _player) "/Game/Animations/Ak3/Ak3_Reload_Montage.Ak3_Reload_Montage"
          (:then
            (Variables|Default|SetReloading true)
            (Animation|Montage|PlayMontage (Variables|Default|GetWeapon) "/Game/Animations/WeaponAnimations/Ak3/Ak3_Weapon_Reload_Montage.Ak3_Weapon_Reload_Montage"
              (:OnBlendOut
                (Variables|Default|SetReloading false))))))
      (:Is%20Not%20Valid
        _))
    (Variables|Default|SetAmmo (Variables|Default|GetMaxAmmo))))

(fn ConstructionScript
  (|CallParentFunction))