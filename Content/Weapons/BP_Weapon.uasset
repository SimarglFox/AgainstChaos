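; BP_Weapon is a weapon Blueprint that plays hand animations for switching and attacking on the owning player.
; Initialize stores the player and hands mesh used by the montages.
; Attack, gated by a cooldown timer, plays the attack montage, immediately fires an empty HitDamageEvent, and subtracts the mana cost from the player.
; HitDamageEvent has no logic here, and mana is not checked before attacking.
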(event Custom|Attack
  (if (not (Variables|Weapon|GetInCooldown))
    (Animation|Montage|PlayMontage (Variables|Default|GetHands) (Variables|Default|GetHandsAttackAnimation)
      (:then
        (CallFunction|HitDamageEvent)
        (Default|SubtractMana (Variables|Default|GetPlayer) (Variables|Weapon|GetManaCost))
        (Utilities|Time|SetTimerbyFunctionName 0 "OnCooldownEnd" (Variables|Weapon|GetCooldown))
        (Variables|Weapon|SetInCooldown true)))))

(event Custom|OnSwich
  (Animation|Montage|PlayMontage (Variables|Default|GetHands) (Variables|Default|GetSwichAnimation)))

(event Custom|HitDamageEvent)

(event Custom|OnCooldownEnd
  (Variables|Weapon|SetInCooldown false))

(fn ConstructionScript)

(fn Initialize
  (params (Player :type First%20Person%20Character%20Object%20Reference) (Hands :type Skeletal%20Mesh%20Component%20Object%20Reference))
  (Variables|Default|SetPlayer Player)
  (Variables|Default|SetHands Hands))