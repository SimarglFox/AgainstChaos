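; Revolver weapon Blueprint, built on a parent class, that fires projectiles and manages its own ammo.
; HitDamageEvent shoots while ammo remains and otherwise reloads; a shot plays the hands montage, spends a round and spawns BP_Bullet after a short delay.
; Bullets start at the Sphere component and face along the weapon's right vector.
; Reload, also run at BeginPlay, refills when the weapon montage blends out, or immediately without a valid Player.
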(event Custom|Shot
  (Animation|Montage|PlayMontage (Variables|/Game/FirstPersonBP/Blueprints/FirstPersonCharacter.FirstPersonCharacter_C|GetHands (Variables|Default|GetPlayer)) "/Game/Animations/Revolver/Revolver_Shot_Montage.Revolver_Shot_Montage"
    (:then
      (Math|Integer|DecrementInt (Variables|Default|GetAmmo)
        (:%20%20
          (Utilities|FlowControl|Delay 0.1)
          (CallFunction|SpawnBullet))))))

(event Custom|Reload
  (bind _player (Variables|Default|GetPlayer))
  (Utilities|IsValid _player
    (:Is%20Valid
      (Animation|Montage|PlayMontage (Variables|/Game/FirstPersonBP/Blueprints/FirstPersonCharacter.FirstPersonCharacter_C|GetHands _player) "/Game/Animations/Revolver/Revolver_Reload_Montage.Revolver_Reload_Montage"
        (:then
          (Animation|Montage|PlayMontage (Variables|Default|GetWeapon) "/Game/Animations/WeaponAnimations/Revolver/Revolver_Weapon_Reload_Montage.Revolver_Weapon_Reload_Montage"
            (:OnBlendOut
              _)))))
    (:Is%20Not%20Valid
      _))
  (Variables|Default|SetAmmo (Variables|Default|GetMaxAmmo)))

(event Custom|SpawnBullet
  (Game|SpawnActorfromClass "/Game/Weapons/Revolver/BP_Bullet.BP_Bullet_C" (Math|Transform|MakeTransform (Transformation|GetWorldLocation (Variables|Default|GetSphere)) (Math|Conversions|RotationFromXVector (Math|Vector|GetRightVector (Variables|Default|GetWeapon)))) "AdjustIfPossibleButDontSpawnIfColliding" self 0) ; Spawn projectile
)

(event EventBeginPlay
  (|CallParentFunction)
  (CallFunction|Reload))

(event EventHitDamageEvent
  (if (> (Variables|Default|GetAmmo) 0)
    (CallFunction|Shot)
    (else
      (CallFunction|Reload))))

(fn ConstructionScript
  (|CallParentFunction))