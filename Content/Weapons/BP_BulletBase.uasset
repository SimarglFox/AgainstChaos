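; BP_BulletBase is a bullet actor that damages what it hits and plays a hit sound at the impact location.
; Its Hit event calls Damage, which casts the bullet's owner to BP_Weapon and applies that weapon's damage value, doing none if the cast fails.
; The bullet then destroys itself only if DestroyBulletOnHit is set.
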(event Custom|Damage
  (params (Target :type Actor%20Object%20Reference))
  (bind _asbp_weapon (Utilities|Casting|CastToBP_Weapon (Components|GetOwner)))
  (Game|Damage|ApplyDamage Target (Variables|/Game/Weapons/BP_Weapon.BP_Weapon_C|GetDamage _asbp_weapon) 0 0))

(event Collision|EventHit
  (params (MyComp :type Primitive%20Component%20Object%20Reference) (Other :type Actor%20Object%20Reference) (OtherComp :type Primitive%20Component%20Object%20Reference) (bSelfMoved :type Boolean) (HitLocation :type Vector :default "0, 0, 0") (HitNormal :type Vector :default "0, 0, 0") (NormalImpulse :type Vector :default "0, 0, 0") (Hit :type Hit%20Result%20Structure%20%28by%20ref%29))
  (CallFunction|Damage Other)
  (Audio|PlaySoundatLocation (Variables|Default|GetHitSound) HitLocation "0, 0, 0" 1.0 1.0 0.0 0 0 0)
  (if (Variables|Default|GetDestroyBulletOnHit)
    (Actor|DestroyActor)))

(fn ConstructionScript)