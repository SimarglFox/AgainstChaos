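; BP_ShotableWeapon is a weapon Blueprint that fires while it has ammo and reloads otherwise.
; HitDamageEvent checks Ammo to call Shot or Reload, and BeginPlay also calls Reload.
; Shot and Reload are empty here, apparently hooks for child Blueprints.
; SpawnBullet spawns a given projectile class at the Sphere component, facing its right vector, with the weapon as owner.
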(event Custom|Shot)

(event Custom|Reload)

(event Custom|SpawnBullet
  (params (Bullet :type Actor%20Class%20Reference))
  (Game|SpawnActorfromClass Bullet (Math|Transform|MakeTransform (Transformation|GetWorldLocation (Variables|Default|GetSphere)) (Math|Conversions|RotationFromXVector (Math|Vector|GetRightVector (Variables|Default|GetSphere)))) "AdjustIfPossibleButDontSpawnIfColliding" self 0) ; Spawn projectile
)

(event EventBeginPlay
  (CallFunction|Reload))

(event Collision|EventActorBeginOverlap
  (params (OtherActor :type Actor%20Object%20Reference)))

(event EventTick
  (params (DeltaSeconds :type Float%20%28single-precision%29)))

(event EventHitDamageEvent
  (if (> (Variables|Default|GetAmmo) 0)
    (CallFunction|Shot)
    (else
      (CallFunction|Reload))))

(fn ConstructionScript
  (|CallParentFunction))