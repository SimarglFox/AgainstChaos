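; Crossbow weapon Blueprint that fires and reloads through montages, extending a parent weapon class.
; It starts reloading on BeginPlay, playing the weapon montage plus a matching hands montage when Player is valid, then flags Reloaded on blend out.
; HitDamageEvent triggers Shot, which requires Reloaded and chains back into Reload when its montage blends out.
; Helper functions toggle Arrow visibility, showing it only while the root is visible.
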(event Custom|Reload
  (bind _player (Variables|Default|GetPlayer))
  (Variables|Default|SetReloading true)
  (Animation|Montage|PlayMontage (Variables|Default|GetWeapon) "/Game/Animations/WeaponAnimations/Crossbow/Crossbow_Weapon_Reload_Montage.Crossbow_Weapon_Reload_Montage"
    (:then
      (Utilities|IsValid _player
        (:Is%20Valid
          (Animation|Montage|PlayMontage (Variables|/Game/FirstPersonBP/Blueprints/FirstPersonCharacter.FirstPersonCharacter_C|GetHands _player) "/Game/Animations/Crossbow/Сrossbow_Reloading_Montage.Сrossbow_Reloading_Montage"))))
    (:OnBlendOut
      (Variables|Default|SetReloading false)
      (Variables|Default|SetReloaded true))))

(event Custom|Shot
  (if (Variables|Default|GetReloaded)
    (Variables|Default|SetShoting true)
    (Animation|Montage|PlayMontage (Variables|Default|GetWeapon) "/Game/Animations/WeaponAnimations/Crossbow/Crossbow_Weapon_Shot_Montage1.Crossbow_Weapon_Shot_Montage1"
      (:OnBlendOut
        (Variables|Default|SetShoting false)
        (CallFunction|Reload)))))

(event EventBeginPlay
  (|CallParentFunction)
  (CallFunction|Reload))

(event EventHitDamageEvent
  (CallFunction|Shot))

(fn ConstructionScript
  (|CallParentFunction))

(fn ActivateArrow
  (if (Variables|/Script/Engine.SceneComponent|GetbVisible (Variables|Default|GetDefaultSceneRoot))
    (Rendering|SetVisibility (Variables|Default|GetArrow) true false)))

(fn DisableArrow
  (Rendering|SetVisibility (Variables|Default|GetArrow) false false))