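; BP_EnemyBase is the base enemy Blueprint, providing movement input, health and death notification.
; AnyDamage feeds TakeDamage, which subtracts from Health and calls the OnDeath dispatcher at zero or below, then prints a debug string.
; Its own OnDeath handler, bound on BeginPlay, removes the enemy from its Spawner's Enemies list and calls the Spawner's Clear when that list empties.
; The actor is not destroyed here.
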(event Custom|Move
  (params (Direction :type Vector) (Scale :type Float%20%28single-precision%29))
  (Pawn|Input|AddMovementInput Direction Scale false))

(event Custom|OnDeath_Event
  (Utilities|IsValid (Variables|Default|GetSpawner)
    (:Is%20Valid
      (Utilities|Array|RemoveItem (Variables|/Game/EnemyBase/SpawnerComponent.SpawnerComponent_C|GetEnemies (Variables|Default|GetSpawner)) self)
      (if (== (Utilities|Array|Length (Variables|/Game/EnemyBase/SpawnerComponent.SpawnerComponent_C|GetEnemies (Variables|Default|GetSpawner))) 0)
        (Default|CallClear (Variables|Default|GetSpawner))))))

(event EventBeginPlay
  (EventDispatchers|BindEventtoOnDeath (delegate Custom|OnDeath_Event)))

(event Game|Damage|EventAnyDamage
  (params (Damage :type Float%20%28single-precision%29) (DamageType :type Damage%20Type%20Object%20Reference) (InstigatedBy :type Controller%20Object%20Reference) (DamageCauser :type Actor%20Object%20Reference))
  (CallFunction|TakeDamage Damage)
  (Development|PrintString "Hello"))

(fn ConstructionScript)

(fn TakeDamage
  (params (Damage :type Float%20%28single-precision%29))
  (bind _output_get (Variables|Default|SetHealth (- (Variables|Default|GetHealth) Damage)))
  (if (<= _output_get 0.0)
    (Default|CallOnDeath)))